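; Level manager for an FPS that tracks remaining enemies, times the run and awards a star rating.
; BeginPlay counts BP_Enemis actors and shows the Time widget, while a one-second Delay on Tick increments the timer.
; When KillEnemi clears the last enemy, time thresholds set the stars saved per level in MyGameInstance, then Menu opens after a pause.
; RespawnPlayer moves the player's capsule to the manager's own location.
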(event Custom|RespawnPlayer
  (bind _returnvalue (Actor|GetActorOfClass "/Game/FPSGame/Blueprints/Actors/BP_Player.BP_Player_C"))
  (bind _asbp_player (Utilities|Casting|CastToBP_Player _returnvalue))
  (Transformation|SetWorldLocation (Variables|/Script/Engine.Character|GetCapsuleComponent _asbp_player) (Transformation|GetActorLocation) false false))

(event Custom|KillEnemi
  (bind _returnvalue (Game|GetGameInstance))
  (bind _time3stars (Variables|Default|Gettime3Stars))
  (bind _timesec (Variables|Default|GettimeSec))
  (bind _timesec_2 (Variables|Default|GettimeSec))
  (bind _output_get (Variables|Default|SetnbEnemisOnLevel (- (Variables|Default|GetnbEnemisOnLevel) 1)))
  (if (<= _output_get 0)
    (if (and (> _timesec 0) (< _timesec _time3stars))
      (Variables|Default|SettextEtoiles "You got 3 stars, Congrats !")
      (bind _asmy_game_instance (Utilities|Casting|CastToMyGameInstance _returnvalue)
        (:then
          (if (Variables|/Game/FPSGame/Blueprints/MyGameInstance.MyGameInstance_C|GetIsLevel2 _asmy_game_instance)
            (Variables|/Game/FPSGame/Blueprints/MyGameInstance.MyGameInstance_C|SetNbStarOnLv2 _asmy_game_instance "3 Stars")
            (else
              (Variables|/Game/FPSGame/Blueprints/MyGameInstance.MyGameInstance_C|SetNbStartOnLv1 _asmy_game_instance "3 Stars"))))
        (:CastFailed
          _))
      (elif (and (>= _timesec_2 _time3stars) (< _timesec_2 (Variables|Default|Gettime2Stars)))
        (Variables|Default|SettextEtoiles "You got 2 stars, Well played !")
        (bind _asmy_game_instance_2 (Utilities|Casting|CastToMyGameInstance _returnvalue)
          (:then
            (if (Variables|/Game/FPSGame/Blueprints/MyGameInstance.MyGameInstance_C|GetIsLevel2 _asmy_game_instance_2)
              (Variables|/Game/FPSGame/Blueprints/MyGameInstance.MyGameInstance_C|SetNbStarOnLv2 _asmy_game_instance_2 "2 Stars")
              (else
                (Variables|/Game/FPSGame/Blueprints/MyGameInstance.MyGameInstance_C|SetNbStartOnLv1 _asmy_game_instance_2 "2 Stars"))))
          (:CastFailed
            _))
        (else
          (Variables|Default|SettextEtoiles "You got 1 star, Try to improve !")
          (bind _asmy_game_instance_3 (Utilities|Casting|CastToMyGameInstance _returnvalue)
            (:then
              (if (Variables|/Game/FPSGame/Blueprints/MyGameInstance.MyGameInstance_C|GetIsLevel2 _asmy_game_instance_3)
                (Variables|/Game/FPSGame/Blueprints/MyGameInstance.MyGameInstance_C|SetNbStarOnLv2 _asmy_game_instance_3 "1 Star")
                (else
                  (Variables|/Game/FPSGame/Blueprints/MyGameInstance.MyGameInstance_C|SetNbStartOnLv1 _asmy_game_instance_3 "1 Star"))))
            (:CastFailed
              _)))))
    (Utilities|FlowControl|Delay 2.0)
    (Game|OpenLevel(byName) "Menu")))

(event EventBeginPlay
  (Utilities|Time|SetGlobalTimeDilation 1.0)
  (bind _outactors (Actor|GetAllActorsOfClass "/Game/FPSGame/Blueprints/Actors/BP_Enemis.BP_Enemis_C"))
  (Variables|Default|SetnbEnemisOnLevel (Utilities|Array|Length _outactors))
  (bind _returnvalue (UserInterface|CreateWidget "/Game/FPSGame/Blueprints/Widgets/Time.Time_C"))
  (UserInterface|Viewport|AddtoViewport _returnvalue 0))

(event EventTick
  (params (DeltaSeconds :type Float%20%28single-precision%29))
  (Utilities|FlowControl|Delay 1.0)
  (Variables|Default|SettimeSec (+ (Variables|Default|GettimeSec) 1)))

(fn ConstructionScript)